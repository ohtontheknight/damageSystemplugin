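; A damage system component that tracks health, death, blocking and invincibility for the actor that owns it.
; TakeDamage runs a CanBeDamage check that routes each hit to block, damage or no damage, with an override flag that bypasses the dead and invincible checks.
; Blocks, deaths and interrupting hits fire dispatchers with damage details for other code to react to.
; Heal restores health up to the maximum while alive.
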(fn `heal`
  (params (amount :type "Float (double-precision)"))
  (returns (`new health` :type "Float (double-precision)"))
  (if (not (`self.isDead`))
    (bind _output_get (set `self.health` (`KismetMathLibrary.FClamp` (+ amount (`self.health`)) 0.0 (`self.maxHealth`))))
    (return _output_get)))

(fn `TakeDamage`
  (params (DamageInfo :type "/damageSystem/S_damage_info Structure") (`damage causer` :type "Actor Object Reference"))
  (returns (wasDamaged :type Boolean))
  (bind (_amount _damagetype _damageresponse _shoulddamageinvincible _canbeblock _canbeparried _shouldforceinterrupt) (break `/damageSystem/S_damage_info` DamageInfo))
  (`self.can be damage` _shoulddamageinvincible _canbeblock
    (:`blockDamage`
      (`self.onblock` _canbeparried `damage causer` _damagetype)
      (return false))
    (:`doDamage`
      (bind _output_get (set `self.health` (- (`self.health`) _amount)))
      (if (<= _output_get 0.0)
        (set `self.isDead` true)
        (`self.onDeath` `damage causer` _damagetype)
        (elif (or (`self.isInterruptable`) _shouldforceinterrupt)
          (`self.onDamageResponse` _damageresponse _damagetype `damage causer`)))
      (return true))
    (:`noDamage`
      (return false))))